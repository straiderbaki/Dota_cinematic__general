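; Firepit prop with an On switch and a jittering component, likely to give the fire a flicker.
; The construction script shows or hides three components based on On, and applies a 40-unit downward offset when off.
; Tick eases a relative location toward a new random point in a box each frame, centered on zero X/Y and the Z captured at BeginPlay.
; This motion runs regardless of On.
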(event `self.ReceiveBeginPlay`
  (set `self.InitialLoc` (.location (`SceneComponent.GetRelativeTransform`))))

(event `self.ReceiveTick`
  (params (DeltaSeconds :type "Float (single-precision)"))
  (`SceneComponent.K2_SetRelativeLocation` (`KismetMathLibrary.VInterpTo` (`SceneComponent.RelativeLocation`) (`KismetMathLibrary.RandomPointInBoundingBox` (`KismetMathLibrary.MakeVector` 0.0 0.0 (.z (`self.InitialLoc`))) (`KismetMathLibrary.MakeVector` 150.0 150.0 40.0)) DeltaSeconds 1.5)))

(fn `UserConstructionScript`
  (if (`self.On?`)
    (`SceneComponent.SetVisibility` true)
    (`SceneComponent.SetVisibility` true)
    (`SceneComponent.SetVisibility` true)
    (`SceneComponent.K2_AddRelativeLocation` (0.0 0.0 0.0) false true)
    (else
      (`SceneComponent.SetVisibility` false)
      (`SceneComponent.SetVisibility` false)
      (`SceneComponent.SetVisibility` false)
      (`SceneComponent.K2_AddRelativeLocation` (0.0 0.0 -40.0) false true))))